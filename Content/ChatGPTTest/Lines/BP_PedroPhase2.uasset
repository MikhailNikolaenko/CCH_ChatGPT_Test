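; BP_PedroPhase2 runs a dialogue encounter in which answers raise or lower Pedro's five-level aggression, leading to win or loss stubs.
; Setup shuffles which response slot is good, neutral or bad, and random getters pull Pedro's line and player responses from the current level's data table row.
; A flat index-keyed boolean map prevents repeats within each level and category, triggering a loss when one runs out.
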(event Custom|SetAggressionLevel
  (params (Correctness :type Integer))
  ;[1 1 1] 0 = Correct, 1 = Neutral, 2 = Incorrect
  (switch int Correctness
    (:0
      (if (== (Variables|Default|GetPedroAggressionLevel) 1)
        (CallFunction|WinningState)
        (else
          (Variables|Default|SetPedroAggressionLevel (- (Variables|Default|GetPedroAggressionLevel) 1)))))
    (:2
      (if (== (Variables|Default|GetPedroAggressionLevel) 5)
        (CallFunction|LosingState)
        (else
          (Variables|Default|SetPedroAggressionLevel (+ (Variables|Default|GetPedroAggressionLevel) 1)))))))

(event Custom|WinningState
  (Development|PrintString "Won"))

(event Custom|LosingState
  (Development|PrintString "Lost"))

(event Custom|Setup
  (Utilities|Array|Shuffle (Variables|Default|GetGoodNeutralBad))
  (Variables|Default|SetCheckIfAnswered false))

(event Custom|Selected
  (params (Response# :type Integer))
  (CallFunction|SetAggressionLevel (Utilities|Array|FindItem (Variables|Default|GetGoodNeutralBad) Response#)))

(event EventBeginPlay
  (bind _lines_columns (Utilities|Struct|MakeLines_Columns "0" "0" "0" "0" "0" "0" "0" "0" "0" "0" "0" "0" "0" "0" "0" "0" "0" "0"))
  (bind _usedlines (Variables|Default|GetUsedLines))
  (Utilities|Array|SetArrayElem _usedlines 0 _lines_columns)
  (Utilities|Array|SetArrayElem _usedlines 1 _lines_columns)
  (Utilities|Array|SetArrayElem _usedlines 2 _lines_columns)
  (Utilities|Array|SetArrayElem _usedlines 3 _lines_columns)
  (Utilities|Array|SetArrayElem _usedlines 4 _lines_columns)
  (CallFunction|FillMap))

(fn ConstructionScript)

(fn PedroRand
  (if (Variables|Default|GetCheckIfAnswered)
    _
    (else
      (bind _returnvalue (Utilities|GetDataTableRow "/Game/ChatGPTTest/Lines/CCHP2_Resp.CCHP2_Resp" (Utilities|Select :Index (- (Variables|Default|GetPedroAggressionLevel) 1) :Option%200 "Level1" :Option%201 "Level2" :Option%202 "Level3" :Option%203 "Level4" :Option%204 "Level5"))
        (:then
          (bind _responseoftypeindex (CallFunction|CheckMap 0 true))
          (CallFunction|UpdateMap 0 _responseoftypeindex true)))))
  (bind _output_get (Variables|Default|SetPedroLastAnswer (Utilities|String|Append (Utilities|Select :Index _responseoftypeindex :Option%200 (.PedroResponse_1 (Utilities|Struct|BreakLines_Columns _returnvalue)) :Option%201 (.PedroResponse_2 (Utilities|Struct|BreakLines_Columns _returnvalue)) :Option%202 (.PedroResponse_3 (Utilities|Struct|BreakLines_Columns _returnvalue)) :Option%203 (.PedroResponse_4 (Utilities|Struct|BreakLines_Columns _returnvalue)) :Option%204 (.PedroResponse_5 (Utilities|Struct|BreakLines_Columns _returnvalue)) :Option%205 (.PedroResponse_6 (Utilities|Struct|BreakLines_Columns _returnvalue)) :Option%206 (.PedroResponse_7 (Utilities|Struct|BreakLines_Columns _returnvalue)) :Option%207 (.PedroResponse_8 (Utilities|Struct|BreakLines_Columns _returnvalue)) :Option%208 (.PedroResponse_9 (Utilities|Struct|BreakLines_Columns _returnvalue))) " " (Utilities|String|ToString(Integer) (Variables|Default|GetPedroAggressionLevel)))))
  (Variables|Default|SetCheckIfAnswered true)
  (return _output_get))

(fn Response1Rand
  (bind _goodneutralbad (Variables|Default|GetGoodNeutralBad))
  (bind _returnvalue (Utilities|Array|FindItem _goodneutralbad 1))
  (bind _returnvalue_2 (Utilities|GetDataTableRow "/Game/ChatGPTTest/Lines/CCHP2_Resp.CCHP2_Resp" (Utilities|Select :Index (- (Variables|Default|GetPedroAggressionLevel) 1) :Option%200 "Level1" :Option%201 "Level2" :Option%202 "Level3" :Option%203 "Level4" :Option%204 "Level5"))
    (:then
      (bind _responseoftypeindex (CallFunction|CheckMap _returnvalue false))
      (CallFunction|UpdateMap _returnvalue _responseoftypeindex false)
      (return (Utilities|Select :Index _returnvalue :Option%200 (Utilities|Select :Index _responseoftypeindex :Option%200 (.Good_1 (Utilities|Struct|BreakLines_Columns _returnvalue_2)) :Option%201 (.Good_2 (Utilities|Struct|BreakLines_Columns _returnvalue_2)) :Option%202 (.Good_3 (Utilities|Struct|BreakLines_Columns _returnvalue_2))) :Option%201 (Utilities|Select :Index _responseoftypeindex :Option%200 (.Neutral_1 (Utilities|Struct|BreakLines_Columns _returnvalue_2)) :Option%201 (.Neutral_2 (Utilities|Struct|BreakLines_Columns _returnvalue_2)) :Option%202 (.Neutral_3 (Utilities|Struct|BreakLines_Columns _returnvalue_2))) :Option%202 (Utilities|Select :Index _responseoftypeindex :Option%200 (.Bad_1 (Utilities|Struct|BreakLines_Columns _returnvalue_2)) :Option%201 (.Bad_2 (Utilities|Struct|BreakLines_Columns _returnvalue_2)) :Option%202 (.Bad_3 (Utilities|Struct|BreakLines_Columns _returnvalue_2))))))))

(fn Response2Rand
  (bind _goodneutralbad (Variables|Default|GetGoodNeutralBad))
  (bind _returnvalue (Utilities|Array|FindItem _goodneutralbad 2))
  (bind _returnvalue_2 (Utilities|GetDataTableRow "/Game/ChatGPTTest/Lines/CCHP2_Resp.CCHP2_Resp" (Utilities|Select :Index (- (Variables|Default|GetPedroAggressionLevel) 1) :Option%200 "Level1" :Option%201 "Level2" :Option%202 "Level3" :Option%203 "Level4" :Option%204 "Level5"))
    (:then
      (bind _responseoftypeindex (CallFunction|CheckMap _returnvalue false))
      (CallFunction|UpdateMap _returnvalue _responseoftypeindex false)
      (return (Utilities|Select :Index _returnvalue :Option%200 (Utilities|Select :Index _responseoftypeindex :Option%200 (.Good_1 (Utilities|Struct|BreakLines_Columns _returnvalue_2)) :Option%201 (.Good_2 (Utilities|Struct|BreakLines_Columns _returnvalue_2)) :Option%202 (.Good_3 (Utilities|Struct|BreakLines_Columns _returnvalue_2))) :Option%201 (Utilities|Select :Index _responseoftypeindex :Option%200 (.Neutral_1 (Utilities|Struct|BreakLines_Columns _returnvalue_2)) :Option%201 (.Neutral_2 (Utilities|Struct|BreakLines_Columns _returnvalue_2)) :Option%202 (.Neutral_3 (Utilities|Struct|BreakLines_Columns _returnvalue_2))) :Option%202 (Utilities|Select :Index _responseoftypeindex :Option%200 (.Bad_1 (Utilities|Struct|BreakLines_Columns _returnvalue_2)) :Option%201 (.Bad_2 (Utilities|Struct|BreakLines_Columns _returnvalue_2)) :Option%202 (.Bad_3 (Utilities|Struct|BreakLines_Columns _returnvalue_2))))))))

(fn Response3Rand
  (bind _goodneutralbad (Variables|Default|GetGoodNeutralBad))
  (bind _returnvalue (Utilities|Array|FindItem _goodneutralbad 3))
  (bind _returnvalue_2 (Utilities|GetDataTableRow "/Game/ChatGPTTest/Lines/CCHP2_Resp.CCHP2_Resp" (Utilities|Select :Index (- (Variables|Default|GetPedroAggressionLevel) 1) :Option%200 "Level1" :Option%201 "Level2" :Option%202 "Level3" :Option%203 "Level4" :Option%204 "Level5"))
    (:then
      (bind _responseoftypeindex (CallFunction|CheckMap _returnvalue false))
      (CallFunction|UpdateMap _returnvalue _responseoftypeindex false)
      (return (Utilities|Select :Index _returnvalue :Option%200 (Utilities|Select :Index _responseoftypeindex :Option%200 (.Good_1 (Utilities|Struct|BreakLines_Columns _returnvalue_2)) :Option%201 (.Good_2 (Utilities|Struct|BreakLines_Columns _returnvalue_2)) :Option%202 (.Good_3 (Utilities|Struct|BreakLines_Columns _returnvalue_2))) :Option%201 (Utilities|Select :Index _responseoftypeindex :Option%200 (.Neutral_1 (Utilities|Struct|BreakLines_Columns _returnvalue_2)) :Option%201 (.Neutral_2 (Utilities|Struct|BreakLines_Columns _returnvalue_2)) :Option%202 (.Neutral_3 (Utilities|Struct|BreakLines_Columns _returnvalue_2))) :Option%202 (Utilities|Select :Index _responseoftypeindex :Option%200 (.Bad_1 (Utilities|Struct|BreakLines_Columns _returnvalue_2)) :Option%201 (.Bad_2 (Utilities|Struct|BreakLines_Columns _returnvalue_2)) :Option%202 (.Bad_3 (Utilities|Struct|BreakLines_Columns _returnvalue_2))))))))

(fn FillMap
  (while (!= (LocalVariables|GetLoop) 90)
    (Utilities|Map|Add (Variables|Default|GetUsedLinesMap) (LocalVariables|GetLoop) false)
    (Math|Integer|IncrementInt (LocalVariables|GetLoop))))

(fn UpdateMap
  (params (ResponseType :type Integer) (ResponseOfTypeIndex :type Integer) (Pedro? :type Boolean))
  (bind _pedroaggressionlevel (Variables|Default|GetPedroAggressionLevel))
  (bind _returnvalue (- _pedroaggressionlevel 1))
  (bind _returnvalue_2 (* _returnvalue 18))
  (Utilities|Map|Add (Variables|Default|GetUsedLinesMap) (select Pedro? (+ (+ _returnvalue_2 9) ResponseOfTypeIndex) (+ (+ (* ResponseType 3) _returnvalue_2) ResponseOfTypeIndex)) true))

(fn CheckMap
  (params (ResponseType :type Integer) (Pedro? :type Boolean))
  (bind _pedroaggressionlevel (Variables|Default|GetPedroAggressionLevel))
  (bind _used (LocalVariables|GetUsed))
  (bind _returnvalue (- _pedroaggressionlevel 1))
  (bind _returnvalue_2 (* _returnvalue 18))
  (while (!= (LocalVariables|GetIterator) (select Pedro? (Class|KismetSystemLibrary|MakeLiteralInteger 9) (Class|KismetSystemLibrary|MakeLiteralInteger 3)))
    (if (.Value (Utilities|Map|Find (Variables|Default|GetUsedLinesMap) (+ (select Pedro? (+ _returnvalue_2 9) (+ (* ResponseType 3) _returnvalue_2)) (LocalVariables|GetIterator))))
      _
      (else
        (Utilities|Array|Add _used (LocalVariables|GetIterator))))
    (Math|Integer|IncrementInt (LocalVariables|GetIterator)))
  (if (Utilities|Array|IsEmpty _used)
    (CallFunction|LosingState)
    (else
      (return (.OutItem (Utilities|Array|Random _used))))))